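; Platform actor that spawns another Platform at a fixed X and Y offset from itself, at the same height, when play begins.
; The spawn runs only while Check is true and Amount is below a limit.
; Check is cleared and Amount incremented only after the spawn call, on the spawning actor, with neither value passed to the new Platform.
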(event EventBeginPlay
  (bind _returnvalue (Transformation|GetActorLocation))
  (if (Variables|Default|GetCheck)
    (if (< (Variables|Default|GetAmount) 10)
      (Game|SpawnActorfromClass "Platform_C" (Math|Transform|MakeTransform (Math|Vector|MakeVector (+ (.x _returnvalue) 2.5e+02) (+ (.y _returnvalue) 1.5e+02) (.z _returnvalue)) "0, 0, 0" "1,1,1") "Undefined" 0 0)
      (Variables|Default|SetCheck false)
      (Variables|Default|SetAmount (+ (Variables|Default|GetAmount) 1)))))

(fn ConstructionScript)